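; AreaWin is a trigger actor that ends the game as a win when anything overlaps its sphere component.
; The overlap, which does not check the other actor, flags PlayerWon on BP_FirstPersonGameMode and clears its AliveTimerHandle and EventHandle timers.
; It then turns off save-on-quit and calls DeleteSave on GI_GameInstance, and disables input on the player pawn.
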(event `self.Sphere1.OnComponentBeginOverlap`
  (params (OverlappedComponent :type "PrimitiveComponent Object Reference") (OtherActor :type "Actor Object Reference") (OtherComp :type "PrimitiveComponent Object Reference") (OtherBodyIndex :type Integer) (bFromSweep :type Boolean) (SweepResult :type "HitResult Structure (by ref)"))
  ; Won Game
  (bind _asgi_game_instance (cast `/Game/Alt_F4/Blueprints/GI_GameInstance` (`GameplayStatics.GetGameInstance`)))
  (bind _asbp_first_person_game_mode (cast `/Game/Alt_F4/Blueprints/BP_FirstPersonGameMode` (`GameplayStatics.GetGameMode`)))
  (set `/Game/Alt_F4/Blueprints/BP_FirstPersonGameMode.PlayerWon` true _asbp_first_person_game_mode)
  (`KismetSystemLibrary.K2_ClearAndInvalidateTimerHandle` (`/Game/Alt_F4/Blueprints/BP_FirstPersonGameMode.AliveTimerHandle` _asbp_first_person_game_mode))
  (`KismetSystemLibrary.K2_ClearAndInvalidateTimerHandle` (`/Game/Alt_F4/Blueprints/BP_FirstPersonGameMode.EventHandle` _asbp_first_person_game_mode))
  (set `/Game/Alt_F4/Blueprints/GI_GameInstance.SaveOnQuit` false _asgi_game_instance)
  (`/Game/Alt_F4/Blueprints/GI_GameInstance.DeleteSave` _asgi_game_instance false)
  (`self.DisableInput` (`GameplayStatics.GetPlayerPawn` 0) null))

(fn `UserConstructionScript`)