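; Game instance that owns the SG_Save slot, persisting player position, rotation and alive time across sessions.
; Init loads or creates the save and can jump straight into MainGame with the HUD, while InitSaveData restores alive time and player transform after a short delay.
; Shutdown copies player state into a fresh save object unless saving is toggled off.
; Dev events, gated by a saved flag, reset, print or suppress saving.
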(event `DevTools`
  (bind _loadedsave (`self.LoadedSave`))
  (if (`self.IsDevToolsEnabled`)
    (set `/Game/Alt_F4/Blueprints/SG_Save.UseDevTools` false _loadedsave)
    (`KismetSystemLibrary.PrintString` "[DevTools] Disabled")
    (else
      (set `/Game/Alt_F4/Blueprints/SG_Save.UseDevTools` true _loadedsave)
      (`KismetSystemLibrary.PrintString` "[DevTools] Enabled"))))

(event `ResetSave`
  ; DevTools: Reset Save
  (if (`self.IsDevToolsEnabled`)
    (`self.DeleteSave` true)
    (`KismetSystemLibrary.PrintString` "[DevTools:Save] Reset")))

(event `self.ReceiveShutdown`
  (bind _player (`self.Player`))
  (bind _loadedsave (`self.LoadedSave`))
  (bind _returnvalue_location (`KismetMathLibrary.BreakTransform` (`Actor.GetTransform` _player)))
  ; Save On Quit
  (if (`self.SaveOnQuit`)
    (set `/Game/Alt_F4/Blueprints/SG_Save.PlayerLastPosition` _returnvalue_location _loadedsave)
    (set `/Game/Alt_F4/Blueprints/SG_Save.PlayerLastRot` (`/Game/Alt_F4/Blueprints/BP_FirstPersonCharacter.Rot` _player) _loadedsave)
    (set `/Game/Alt_F4/Blueprints/SG_Save.AliveTime` (`self.PlayerAliveTime`) _loadedsave)
    (`self.SaveData` _loadedsave)))

(event `self.ReceiveInit`
  ; Init
  ; Load Save
  (bind _savefound (`self.GetLoadSave` :!label _label))
  (bind _output_get (set `self.LoadedSave` _savefound))
  ; Direct Open & Begin Play
  (if (`/Game/Alt_F4/Blueprints/SG_Save.LoadDirectToGame` (`self.LoadedSave`))
    (`GameplayStatics.OpenLevel` "MainGame")
    (`KismetSystemLibrary.Delay` 0.01)
    (bind _asbp_first_person_game_mode (cast `/Game/Alt_F4/Blueprints/BP_FirstPersonGameMode` (`GameplayStatics.GetGameMode`)))
    (`/Game/Alt_F4/Blueprints/BP_FirstPersonGameMode.BeginGame` _asbp_first_person_game_mode)
    (set `PlayerController.bShowMouseCursor` false (`GameplayStatics.GetPlayerController` 0))
    (`WidgetLayoutLibrary.RemoveAllWidgets`)
    (bind _returnvalue (`|CreateWidget` "/Game/Alt_F4/Blueprints/UI_HUD.UI_HUD_C"))
    (`UserWidget.AddToViewport` _returnvalue 0)))

(event `FullInit`
  ; Init
  (`|ExecutionSequence`
    (:`then_0`
      (goto _label))
    (:`then_1`
      (`|ExecutionSequence` :!label _label_2
        (:`then_0`
          ; Set Alive Time
          (set `self.PlayerAliveTime` (`/Game/Alt_F4/Blueprints/SG_Save.AliveTime` (stale `self.ReceiveInit` _output_get)))
          ; Dev Tools Notification
          (if (`self.IsDevToolsEnabled`)
            (`KismetSystemLibrary.PrintString` "[DeveloperTools] Enabled")))
        (:`then_1`
          ; Set Player
          (`KismetSystemLibrary.Delay` 0.2)
          (bind _asbp_first_person_character (cast `/Game/Alt_F4/Blueprints/BP_FirstPersonCharacter` (`GameplayStatics.GetPlayerPawn` 0)))
          (bind _output_get (set `self.Player` _asbp_first_person_character))
          (bind _playerlastposition (`/Game/Alt_F4/Blueprints/SG_Save.PlayerLastPosition` (stale `self.ReceiveInit` _output_get)))
          ; Set Players Prev. Pos
          (if (not (`KismetMathLibrary.Vector_IsZero` _playerlastposition))
            (`Actor.K2_SetActorLocation` _output_get _playerlastposition false false))
          ; Set Players Prev. Rot
          (`Controller.SetControlRotation` (`Pawn.GetController` _output_get) (`/Game/Alt_F4/Blueprints/SG_Save.PlayerLastRot` (stale `self.ReceiveInit` _output_get))))))))

(event `ShowSaveValues`
  (bind _loadedsave (`self.LoadedSave`))
  ; DevTools: Show Save Values
  (if (`self.IsDevToolsEnabled`)
    (`|ExecutionSequence`
      (:`then_0`
        (`KismetSystemLibrary.PrintString` (`KismetStringLibrary.Concat_StrStr` "[DevTools:Save:AliveTime] " (`KismetStringLibrary.Conv_DoubleToString` (`/Game/Alt_F4/Blueprints/SG_Save.AliveTime` _loadedsave)))))
      (:`then_1`
        (`KismetSystemLibrary.PrintString` (`KismetStringLibrary.Concat_StrStr` "[DevTools:Save:DiedBeforeF4] " (`KismetStringLibrary.Conv_BoolToString` (`/Game/Alt_F4/Blueprints/SG_Save.DiedBeforeF4` _loadedsave)))))
      (:`then_2`
        (`KismetSystemLibrary.PrintString` (`KismetStringLibrary.Concat_StrStr` "[DevTools:Save:PlayerLastPosition] " (`KismetStringLibrary.Conv_VectorToString` (`/Game/Alt_F4/Blueprints/SG_Save.PlayerLastPosition` _loadedsave)))))
      (:`then_3`
        (`KismetSystemLibrary.PrintString` (`KismetStringLibrary.Concat_StrStr` "[DevTools:Save:PlayerLastRot] " (`KismetStringLibrary.Conv_RotatorToString` (`/Game/Alt_F4/Blueprints/SG_Save.PlayerLastRot` _loadedsave))))))))

(event `InitSaveData`
  ; Init Save Data
  (goto _label_2))

(event `DontSave`
  ; DevTools: Reset Save
  (if (`self.IsDevToolsEnabled`)
    (if (`self.SaveOnQuit`)
      (set `self.SaveOnQuit` false)
      (`KismetSystemLibrary.PrintString` "[DevTools:SaveOnReset] True")
      (else
        (set `self.SaveOnQuit` true)
        (`KismetSystemLibrary.PrintString` "[DevTools:SaveOnReset] False")))))

(fn `DeleteSave`
  (params (DoFullReInit :type Boolean :default true))
  ; Delete Save
  (`GameplayStatics.DeleteGameInSlot` (`self.SaveName`))
  (if DoFullReInit
    (`self.FullInit`))
  (return))

(fn `GetLoadSave`
  (returns (SaveFound :type "/Game/Alt_F4/Blueprints/SG_Save Object Reference"))
  ; Try Get Save
  (bind _returnvalue (`GameplayStatics.LoadGameFromSlot` (`self.SaveName`)))
  (if (`KismetSystemLibrary.IsValid` _returnvalue)
    ; Load Save
    (bind _assg_save (cast `/Game/Alt_F4/Blueprints/SG_Save` _returnvalue))
    (`KismetSystemLibrary.PrintString` "Loaded Save!")
    (return _assg_save)
    (else
      ; Create Save
      (bind _returnvalue_2 (`GameplayStatics.CreateSaveGameObject` "/Game/Alt_F4/Blueprints/SG_Save.SG_Save_C"))
      (`self.Save` _returnvalue_2)
      (`KismetSystemLibrary.PrintString` "Created Save!")
      (return _returnvalue_2))))

(fn `IsDevToolsEnabled`
  (returns (isEnabled :type Boolean))
  ; Is Dev Tools Enabled
  (return (`/Game/Alt_F4/Blueprints/SG_Save.UseDevTools` (`self.LoadedSave`))))

(fn `Save`
  (params (Save :type "/Game/Alt_F4/Blueprints/SG_Save Object Reference"))
  ; Save Game To File
  (`GameplayStatics.SaveGameToSlot` Save (`self.SaveName`))
  (return))

(fn `SaveData`
  (params (Save :type "/Game/Alt_F4/Blueprints/SG_Save Object Reference"))
  ; Save Game Data
  (bind _returnvalue (`GameplayStatics.CreateSaveGameObject` "/Game/Alt_F4/Blueprints/SG_Save.SG_Save_C"))
  (set `/Game/Alt_F4/Blueprints/SG_Save.AliveTime` (`/Game/Alt_F4/Blueprints/SG_Save.AliveTime` Save) _returnvalue)
  (set `/Game/Alt_F4/Blueprints/SG_Save.DiedBeforeF4` (`/Game/Alt_F4/Blueprints/SG_Save.DiedBeforeF4` Save) _returnvalue)
  (set `/Game/Alt_F4/Blueprints/SG_Save.PlayerLastPosition` (`/Game/Alt_F4/Blueprints/SG_Save.PlayerLastPosition` Save) _returnvalue)
  (set `/Game/Alt_F4/Blueprints/SG_Save.PlayerLastRot` (`/Game/Alt_F4/Blueprints/SG_Save.PlayerLastRot` Save) _returnvalue)
  (set `/Game/Alt_F4/Blueprints/SG_Save.UseDevTools` (`/Game/Alt_F4/Blueprints/SG_Save.UseDevTools` Save) _returnvalue)
  (set `/Game/Alt_F4/Blueprints/SG_Save.LoadDirectToGame` (`/Game/Alt_F4/Blueprints/SG_Save.LoadDirectToGame` Save) _returnvalue)
  (`self.Save` _returnvalue)
  (return))